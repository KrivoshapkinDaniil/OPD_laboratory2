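; Inventory key item, named for a wood door, that the player picks up and uses on key-locked doors.
; Interacting with it sends it to the player's inventory.
; Using it casts the character interact component's current target to BP_DoorKey, then runs the parent use logic and calls OpenDoor on that component with the KeyID from the item's data asset.
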(event `/Game/ResidentHorrorV1/Blueprints/BP_Interact/BPI_Interact.Interact Item`
  (params (ACTO :type "Actor Object Reference") (Player :type "/Game/ResidentHorrorV1/Character/BP_Character/BP_Resident_HorrorV1 Object Reference"))
  ;[0 0 0] Add item In Inventory
  (`self.Send Item To Inventory` Player Player))

(fn `UseItem`
  (returns (Sucess :type Boolean))
  (bind _interact (`/Game/ResidentHorrorV1/Blueprints/BP_Interact/BPC_Interact.Interact` (`/Game/ResidentHorrorV1/Character/BP_Character/BP_Resident_HorrorV1.BPC_Interact` (`/Game/ResidentHorrorV1/Blueprints/BP_FunctionLibray/BPFL_LibrayCharacter.My character Resident Horror`))))
  (bind _asbp_door_key (cast `/Game/ResidentHorrorV1/Blueprints/BP_Door/BaseDoor/BP_DoorKey` _interact))
  (`/Engine/EditorBlueprintResources/StandardMacros.IsValid` _interact
    (:`Is Valid`
      (if (== (`/Game/ResidentHorrorV1/Blueprints/BP_Interact/BPC_Interact.Interact` (`/Game/ResidentHorrorV1/Character/BP_Character/BP_Resident_HorrorV1.BPC_Interact` (`/Game/ResidentHorrorV1/Blueprints/BP_FunctionLibray/BPFL_LibrayCharacter.My character Resident Horror`))) _asbp_door_key)
        (bind _sucess (`parent.UseItem`))
        (`/Game/ResidentHorrorV1/Blueprints/BP_Interact/BPC_Interact.Open Door` (`/Game/ResidentHorrorV1/Character/BP_Character/BP_Resident_HorrorV1.BPC_Interact` (`/Game/ResidentHorrorV1/Blueprints/BP_FunctionLibray/BPFL_LibrayCharacter.My character Resident Horror`)) (`/Game/ResidentHorrorV1/Blueprints/BP_Inventory/DA_BaseInteract.KeyID` (`.DA_BaseInteract_112_E5D63A474E86D51C38EA9ABF9499DC91` (break `/Game/ResidentHorrorV1/Blueprints/BP_Inventory/S_Item_Structure` (`.ItemStructure_3_D962DD8B4106829899F7C99F3F34F837` (break `/Game/ResidentHorrorV1/Blueprints/BP_Inventory/S_SlotStruct` (`self.S ItemStrucuture`)))))))
        (return _sucess)))))

(fn `UserConstructionScript`
  (`parent.UserConstructionScript`))